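; WeaponPickup is a pickup actor that grants a weapon or ammo to a player character that overlaps its collision.
; It accepts Rocco_PlayerCharacter or Aaron_PlayerCharacter, running the same logic in a separate cast branch for each.
; If WeaponType is already in the character's WeaponsAvailable, it calls GiveAmmo; otherwise it calls GiveWeapon with the ammo amount.
; The pickup then destroys itself.
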(event OnComponentBeginOverlap(Collision)
  (params (OverlappedComponent :type Primitive%20Component%20Object%20Reference) (OtherActor :type Actor%20Object%20Reference) (OtherComp :type Primitive%20Component%20Object%20Reference) (OtherBodyIndex :type Integer) (bFromSweep :type Boolean) (SweepResult :type Hit%20Result%20Structure%20%28by%20ref%29))
  (bind _weapontype (Variables|Default|GetweaponType))
  (bind _ammoamount (Variables|Default|GetammoAmount))
  (bind _weapontype_2 (Variables|Default|GetweaponType))
  (bind _ammoamount_2 (Variables|Default|GetammoAmount))
  (bind _asrocco_player_character (Utilities|Casting|CastToRocco_PlayerCharacter OtherActor)
    (:then
      (bind _index (Utilities|FlowControl|ForLoopwithBreak 0 (- (Utilities|Array|Length (Variables|/Game/RoccoStuff/Rocco_PlayerCharacter.Rocco_PlayerCharacter_C|GetweaponsAvailable _asrocco_player_character)) 1) :!label _label)
        (:LoopBody
          (if (Utilities|Enum|Equal(Enum) (Utilities|Array|Get(acopy) (Variables|/Game/RoccoStuff/Rocco_PlayerCharacter.Rocco_PlayerCharacter_C|GetweaponsAvailable _asrocco_player_character) _index) _weapontype_2)
            (Default|GiveAmmo _asrocco_player_character _weapontype_2 _ammoamount_2)
            (Variables|Default|SetammoApplied true)
            (goto _label Break)))
        (:Completed
          (if (Variables|Default|GetammoApplied)
            _
            (else
              (Default|GiveWeapon _asrocco_player_character _weapontype_2 _ammoamount_2)))
          (Actor|DestroyActor))))
    (:CastFailed
      (bind _asaaron_player_character (Utilities|Casting|CastToAaron_PlayerCharacter OtherActor))
      (bind _index_2 (Utilities|FlowControl|ForLoopwithBreak 0 (- (Utilities|Array|Length (Variables|/Game/AaronStuff/Blueprints/Aaron_PlayerCharacter.Aaron_PlayerCharacter_C|GetweaponsAvailable _asaaron_player_character)) 1) :!label _label_2)
        (:LoopBody
          (if (Utilities|Enum|Equal(Enum) (Utilities|Array|Get(acopy) (Variables|/Game/AaronStuff/Blueprints/Aaron_PlayerCharacter.Aaron_PlayerCharacter_C|GetweaponsAvailable _asaaron_player_character) _index_2) _weapontype)
            (Default|GiveAmmo _asaaron_player_character _weapontype _ammoamount)
            (Variables|Default|SetammoApplied true)
            (goto _label_2 Break)))
        (:Completed
          (if (Variables|Default|GetammoApplied)
            _
            (else
              (Default|GiveWeapon _asaaron_player_character _weapontype _ammoamount)))
          (Actor|DestroyActor))))))

(fn ConstructionScript)