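; Rocket projectile that flies straight ahead and explodes on overlap.
; Tick moves the root along its forward vector at constant speed without sweeping.
; A mesh overlap outside the first custom collision channel hides the mesh, fires a radial impulse and plays a pitch-randomized sound, then destroys the actor after the sound's duration.
; The Hit guard is only ever set false, so it does not block repeat overlaps.
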(event OnComponentBeginOverlap(rocketMesh)
  (params (OverlappedComponent :type Primitive%20Component%20Object%20Reference) (OtherActor :type Actor%20Object%20Reference) (OtherComp :type Primitive%20Component%20Object%20Reference) (OtherBodyIndex :type Integer) (bFromSweep :type Boolean) (SweepResult :type Hit%20Result%20Structure%20%28by%20ref%29))
  (bind _explodesfx (Variables|Default|GetexplodeSFX))
  (if (and (Utilities|Enum|NotEqual(Enum) (Collision|GetCollisionObjectType OtherComp) "ECC_GameTraceChannel1") (Math|Boolean|NotEqual(Boolean) (Variables|Default|Gethit) true))
    (Variables|Default|Sethit false)
    (Rendering|SetVisibility (Variables|Default|GetrocketMesh) false false)
    (Class|RadialForceComponent|FireImpulse (Variables|Default|GetradialForce))
    (Audio|PlaySoundatLocation _explodesfx (Transformation|GetWorldLocation (Variables|Default|GetDefaultSceneRoot)) "0, 0, 0" 1.0 (Math|Random|RandomFloatinRange 0.9 1.1) 0.0 0 0 0)
    (Utilities|FlowControl|Delay (Variables|/Script/Engine.SoundBase|GetDuration _explodesfx))
    (Actor|DestroyActor)))

(event EventTick
  (params (DeltaSeconds :type Float%20%28single-precision%29))
  (bind _defaultsceneroot (Variables|Default|GetDefaultSceneRoot))
  (Transformation|SetWorldLocation (Variables|Default|GetDefaultSceneRoot) (+ (Transformation|GetWorldLocation _defaultsceneroot) (* (Math|Vector|GetForwardVector _defaultsceneroot) (* DeltaSeconds 2e+03))) false false))

(fn ConstructionScript)