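; Ranged enemy that hunts the player and fires DusterProjectiles, destroying itself on death.
; Each Tick, a line trace sets Aggro on a visible player, or Idle when blocked or invisible, moving to the last seen location.
; Aggro chases until within shooting range, then changes speed, moves to random trace-checked points around the player and launches physics-velocity projectiles.
; Repositioning and firing use frame-counted timers.
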(event Custom|OnDeath
  (Actor|DestroyActor))

(event EventBeginPlay
  (EventDispatchers|BindEventtoEnemyDied (delegate Custom|OnDeath))
  (|CallParentFunction)
  (Variables|Default|SetTarget (Game|Player|GetPlayerPawn 0)))

(event EventTick
  (params (DeltaSeconds :type Float%20%28single-precision%29))
  (|CallParentFunction DeltaSeconds)
  (if (not (Variables|Default|GetIsDead))
    (bind _outhit (CallFunction|LineTracetoTarget))
    (bind _asaaron_player_character (Utilities|Casting|CastToplayerCharacter (.hitactor _outhit))
      (:then
        (if (Variables|/Game/Blueprints/Player/playerCharacter.playerCharacter_C|GetisInvisible _asaaron_player_character)
          (Variables|Default|SetCanSeePlayer false :!label _label)
          (Variables|Default|SetState "NewEnumerator0")
          (else
            (Variables|Default|SetCanSeePlayer true)
            (Variables|Default|SetState "NewEnumerator1"))))
      (:CastFailed
        (goto _label)))
    (switch Utilities|FlowControl|Switch|SwitchonEnemyState (Variables|Default|GetState)
      (:NewEnumerator0
        (AI|AIMoveTo 0 (Variables|Default|GetLastSeenTargetLocation) 0 5.0 false))
      (:NewEnumerator1
        (Variables|Default|SetLastSeenTargetLocation (Transformation|GetWorldLocation (Variables|/Script/Engine.Actor|GetRootComponent (Variables|Default|GetTarget))))
        (if (<= (Variables|Default|GetDistanceToTarget) (Variables|Default|GetShootingDistance))
          (Math|Integer|DecrementInt (Variables|Default|GetRandomDestinationTimer)
            (:%20%20
              (if (<= (Variables|Default|GetRandomDestinationTimer) 0)
                (CallFunction|SetNewPathfindDestination)
                (Variables|Default|SetRandomDestinationTimer 500))
              (AI|AIMoveTo self (Variables|Default|GetPathfindDestination) 0 5.0 false
                (:then
                  _)
                (:OnSuccess
                  (CallFunction|LookatTarget)))
              (Variables|/Script/Engine.CharacterMovementComponent|SetMaxWalkSpeed (Variables|Character|GetCharacterMovement) (Variables|Default|GetInRangeMovementSpeed))
              (if (<= (Variables|Default|GetFireProjectileTimer) 0)
                (CallFunction|FireProjectile)
                (Variables|Default|SetFireProjectileTimer 260))
              (Math|Integer|DecrementInt (Variables|Default|GetFireProjectileTimer))))
          (else
            (AI|AIMoveTo self "0, 0, 0" (Variables|Default|GetTarget) 0.0 false
              (:then
                _)
              (:OnSuccess
                (CallFunction|LookatTarget)))
            (Variables|/Script/Engine.CharacterMovementComponent|SetMaxWalkSpeed (Variables|Character|GetCharacterMovement) (Variables|Default|GetOutOfRangeMovementSpeed))))))))

(fn ConstructionScript
  (|CallParentFunction))

(fn LineTracetoTarget
  (bind _capsulecomponent (Variables|Default|GetCapsuleComponent))
  (bind _target (Variables|Default|GetTarget))
  (bind _returnvalue (Transformation|GetWorldLocation _capsulecomponent))
  (bind _rootcomponent (Variables|/Script/Engine.Actor|GetRootComponent _target))
  (bind _returnvalue_2 (Transformation|GetWorldLocation _rootcomponent))
  (Variables|Default|SetDistanceToTarget (Math|Vector|Distance(Vector) _returnvalue _returnvalue_2))
  (bind (_outhit _returnvalue_3) (Collision|LineTraceByChannel _returnvalue _returnvalue_2 "TraceTypeQuery2" false 0 "None"))
  (return _outhit _returnvalue_3))

(fn FireProjectile
  (bind _capsulecomponent (Variables|Default|GetCapsuleComponent))
  (bind _target (Variables|Default|GetTarget))
  (bind _returnvalue (Transformation|GetWorldLocation _capsulecomponent))
  (bind _rootcomponent (Variables|/Script/Engine.Actor|GetRootComponent _target))
  (bind _returnvalue_2 (Transformation|GetWorldLocation _rootcomponent))
  (bind _returnvalue_3 (Game|SpawnActorfromClass "/Game/Blueprints/Enemies/Projectiles/DusterProjectile.DusterProjectile_C" (Math|Transform|MakeTransform _returnvalue (Math|Rotator|FindLookatRotation _returnvalue _returnvalue_2) "1,1,1") "AlwaysSpawn" 0 0))
  (Physics|SetPhysicsLinearVelocity (Variables|/Game/Blueprints/Enemies/Projectiles/DusterProjectile.DusterProjectile_C|GetSphere _returnvalue_3) (* (Math|Vector|GetUnitDirection(Vector) _returnvalue _returnvalue_2) (Variables|Default|GetProjectileSpeed)) false "None"))

(fn SetNewPathfindDestination
  (bind _returnvalue (Math|Random|RandomUnitVector))
  (bind _target (Variables|Default|GetTarget))
  (bind _pathfindingvariancemulti (Variables|Default|GetPathfindingVarianceMulti))
  (bind _returnvalue_2 (* (Math|Vector|MakeVector (.x _returnvalue) (.y _returnvalue) 0.0) _pathfindingvariancemulti))
  (bind _rootcomponent (Variables|/Script/Engine.Actor|GetRootComponent _target))
  (bind _returnvalue_3 (Transformation|GetWorldLocation _rootcomponent))
  (bind _returnvalue_4 (+ _returnvalue_3 _returnvalue_2))
  (Utilities|FlowControl|ForLoopwithBreak 0 0 :!label _label
    (:LoopBody
      (bind _returnvalue_5 (Collision|LineTraceByChannel _returnvalue_4 _returnvalue_3 "TraceTypeQuery1" false 0 "None"))
      (if _returnvalue_5
        (bind _result (Math|Integer|IncrementInt (LocalVariables|Getcycles))
          (:%20%20
            (if (> _result 20)
              (goto _label Break))))
        (else
          (Variables|Default|SetPathfindDestination _returnvalue_4)
          (return))))
    (:Completed
      (return))))