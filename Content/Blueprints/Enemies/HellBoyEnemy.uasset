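; HellBoyEnemy is a melee enemy that chases and punches the player, then stops on death and is destroyed after a delay.
; Each Tick, a line trace to the player sets Idle or Aggro, treating invisible players as unseen.
; In Aggro, AIMoveTo closes in, and frame-counted timers gate and time punches that damage players overlapping PunchBox.
; JumpAtTarget is an empty stub with disconnected impulse logic.
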(event Custom|OnDeath
  (Utilities|FlowControl|Delay 3.0)
  (Development|PrintString "Hello")
  (Actor|DestroyActor))

(event EventTick
  (params (DeltaSeconds :type Float%20%28single-precision%29))
  (|CallParentFunction DeltaSeconds)
  (if (Variables|Default|GetIsDead)
    (Class|NavMovementComponent|StopActiveMovement (Variables|Character|GetCharacterMovement))
    (else
      (if (Variables|Default|GetPunching)
        (Math|Integer|IncrementInt (Variables|Default|GetPunchDuration)
          (:%20%20
            _)))
      ;[1 1 1] AI
      (bind _outhit (CallFunction|LineTracetoTarget))
      (bind _asaaron_player_character (Utilities|Casting|CastToplayerCharacter (.hitactor _outhit))
        (:then
          (if (Variables|/Game/Blueprints/Player/playerCharacter.playerCharacter_C|GetisInvisible _asaaron_player_character)
            (Variables|Default|SetCanSeePlayer false :!label _label)
            (Variables|Default|SetState "NewEnumerator0")
            (else
              (Variables|Default|SetCanSeePlayer true)
              (Variables|Default|SetState "NewEnumerator1"))))
        (:CastFailed
          (goto _label)))
      (switch Utilities|FlowControl|Switch|SwitchonEnemyState (Variables|Default|GetState)
        (:NewEnumerator0
          (AI|AIMoveTo 0 "0, 0, 0" 0 5.0 false))
        (:NewEnumerator1
          (Math|Integer|DecrementInt (Variables|Default|GetTimerUntilPunch)
            (:%20%20
              (bind _output_get (Variables|Default|SetLastSeenTargetLocation (Transformation|GetWorldLocation (Variables|/Script/Engine.Actor|GetRootComponent (Variables|Default|GetTarget)))))
              (AI|AIMoveTo self _output_get 0 1.2e+02 false
                (:then
                  (if (and (<= (Variables|Default|GetTimerUntilPunch) 0) (<= (Variables|Default|GetDistanceToTarget) (Variables|Default|GetPunchingDistance)))
                    (Variables|Default|SetPunching true)
                    (Variables|Default|SetTimerUntilPunch 70)
                    (if (== (Variables|Default|GetPunchDuration) 8) :!label _label_2
                      (CallFunction|Punch))
                    (if (>= (Variables|Default|GetPunchDuration) (Variables|Default|GetPunchMaxDuration))
                      (Variables|Default|SetPunching false)
                      (Variables|Default|SetPunchDuration 0))
                    (elif (Variables|Default|GetPunching)
                      (goto _label_2))))))))))))

(event EventBeginPlay
  (EventDispatchers|BindEventtoEnemyDied (delegate Custom|OnDeath))
  (Variables|Default|SetTarget (Game|Player|GetPlayerPawn 0)))

(fn ConstructionScript
  (|CallParentFunction))

(fn LineTracetoTarget
  (bind _capsulecomponent (Variables|Default|GetCapsuleComponent))
  (bind _target (Variables|Default|GetTarget))
  (bind _returnvalue (Transformation|GetWorldLocation _capsulecomponent))
  (bind _rootcomponent (Variables|/Script/Engine.Actor|GetRootComponent _target))
  (bind _returnvalue_2 (Transformation|GetWorldLocation _rootcomponent))
  (Variables|Default|SetDistanceToTarget (Math|Vector|Distance(Vector) _returnvalue _returnvalue_2))
  (bind (_outhit _returnvalue_3) (Collision|LineTraceByChannel _returnvalue _returnvalue_2 "TraceTypeQuery2" false 0 "None"))
  (return _outhit _returnvalue_3))

(fn JumpatTarget)

(fn Punch
  (for _array_element (Class|PrimitiveComponent|GetOverlappingComponents (Variables|Default|GetPunchBox))
    (bind _asaaron_player_character (Utilities|Casting|CastToplayerCharacter (Components|GetOwner _array_element)))
    (Default|TakeDamage _asaaron_player_character 25)
    (Development|PrintString "Hello")))