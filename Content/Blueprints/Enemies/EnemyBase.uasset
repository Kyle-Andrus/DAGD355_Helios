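; EnemyBase is an enemy Blueprint that provides health, damage, death notification and target facing.
; Health starts at MaxHealth, and TakeDamage subtracts flat damage plus a fraction of MaxHealth, then calls TakenDamage with the amount lost.
; Tick polls for zero health and uses DoOnce to call EnemyDied a single time.
; LookAtTarget rotates the capsule toward Target using only X and Y positions.
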(event EventBeginPlay
  (Variables|Default|SetHealth (Variables|Default|GetMaxHealth)))

(event EventTick
  (params (DeltaSeconds :type Float%20%28single-precision%29))
  ;[1 1 1] Set is dead
  (Variables|Default|SetIsDead (<= (Variables|Default|GetHealth) 0.0))
  ;[1 1 1] is dead?
  (if (Variables|Default|GetIsDead)
    (Utilities|FlowControl|DoOnce false
      (:Completed
        ;[1 1 1] Die
        (Default|CallEnemyDied)))))

(fn ConstructionScript)

(fn TakeDamage
  (params (Damage :type Float%20%28single-precision%29) (Percent :type Float%20%28single-precision%29))
  (LocalVariables|SetHealthBeforeDamage (Variables|Default|GetHealth))
  (bind _output_get (Variables|Default|SetHealth (- (Variables|Default|GetHealth) (+ Damage (* Percent (Variables|Default|GetMaxHealth))))))
  (Default|CallTakenDamage (- (LocalVariables|GetHealthBeforeDamage) _output_get)))

(fn LookatTarget
  (bind _target (Variables|Default|GetTarget))
  (bind _capsulecomponent (Variables|Collision|GetCapsuleComponent))
  (bind _returnvalue (Transformation|GetWorldLocation _capsulecomponent))
  (bind _rootcomponent (Variables|/Script/Engine.Actor|GetRootComponent _target))
  (bind _returnvalue_2 (Transformation|GetWorldLocation _rootcomponent))
  (Transformation|SetWorldRotation (Variables|Collision|GetCapsuleComponent) (Math|Rotator|FindLookatRotation (Math|Vector|MakeVector (.x _returnvalue) (.y _returnvalue) 0.0) (Math|Vector|MakeVector (.x _returnvalue_2) (.y _returnvalue_2) 0.0)) false false))