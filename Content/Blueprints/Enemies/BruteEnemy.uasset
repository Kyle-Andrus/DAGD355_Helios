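; Brute enemy that chases the player and fires projectile volleys when in range, destroying itself on death.
; Each Tick, a line trace to the player sets Aggro on sight, or Idle if blocked or the player is invisible.
; In Aggro it moves directly toward a distant player; within shooting distance it switches speed and follows periodically randomized offsets around them.
; Volley, shot and reposition timers count ticks rather than seconds, so their timing depends on frame rate.
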(event Custom|OnDeath
  (Actor|DestroyActor))

(event EventBeginPlay
  (EventDispatchers|BindEventtoEnemyDied (delegate Custom|OnDeath))
  (|CallParentFunction)
  (Variables|Default|SetTarget (Game|Player|GetPlayerPawn 0)))

(event EventTick
  (params (DeltaSeconds :type Float%20%28single-precision%29))
  (bind _returnvalue (Math|Random|RandomUnitVector))
  (|CallParentFunction DeltaSeconds)
  (if (not (Variables|Default|GetIsDead))
    (bind _outhit (CallFunction|LineTracetoTarget))
    (bind _asaaron_player_character (Utilities|Casting|CastToplayerCharacter (.hitactor _outhit))
      (:then
        (if (Variables|/Game/Blueprints/Player/playerCharacter.playerCharacter_C|GetisInvisible _asaaron_player_character)
          (Variables|Default|SetCanSeePlayer false :!label _label)
          (Variables|Default|SetState "NewEnumerator0")
          (else
            (Variables|Default|SetCanSeePlayer true)
            (Variables|Default|SetState "NewEnumerator1"))))
      (:CastFailed
        (goto _label)))
    (switch Utilities|FlowControl|Switch|SwitchonEnemyState (Variables|Default|GetState)
      (:NewEnumerator1
        ;[1 1 1] Aggro AI
        (if (<= (Variables|Default|GetDistanceToTarget) (Variables|Default|GetShootingDistance))
          (Math|Integer|DecrementInt (Variables|Default|GetRandomDestinationTimer)
            (:%20%20
              (Math|Integer|DecrementInt (Variables|Default|GetFireVolleyTimer)
                (:%20%20
                  (if (<= (Variables|Default|GetRandomDestinationTimer) 0)
                    (bind _output_get (Variables|Default|SetRandomDestinationOffset (* (Math|Vector|MakeVector (.x _returnvalue) (.y _returnvalue) 0.0) (Variables|Default|GetPathfindingVarianceMulti))))
                    (Variables|Default|SetRandomDestinationTimer 180))
                  (AI|AIMoveTo self (+ _output_get (Transformation|GetWorldLocation (Variables|/Script/Engine.Actor|GetRootComponent (Variables|Default|GetTarget)))) 0 0.0 false
                    (:then
                      _)
                    (:OnSuccess
                      (CallFunction|LookatTarget)))
                  (Variables|/Script/Engine.CharacterMovementComponent|SetMaxWalkSpeed (Variables|Character|GetCharacterMovement) (Variables|Default|GetInRangeMovementSpeed))
                  (if (<= (Variables|Default|GetFireVolleyTimer) 0)
                    (Variables|Default|SetFiringVolley true)
                    (Variables|Default|SetFireVolleyTimer 260)
                    (Variables|Default|SetVolleyCount 0))
                  (if (Variables|Default|GetFiringVolley)
                    (if (<= (Variables|Default|GetFireProjectileTimer) 0)
                      (CallFunction|FireProjectile)
                      (Math|Integer|IncrementInt (Variables|Default|GetVolleyCount)
                        (:%20%20
                          _)))
                    (Math|Integer|DecrementInt (Variables|Default|GetFireProjectileTimer)
                      (:%20%20
                        (if (>= (Variables|Default|GetVolleyCount) (Variables|Default|GetMaxVolleyCount))
                          (Variables|Default|SetFiringVolley false)))))))))
          (else
            (AI|AIMoveTo self "0, 0, 0" (Variables|Default|GetTarget) 0.0 false
              (:then
                _)
              (:OnSuccess
                (CallFunction|LookatTarget)))
            (Variables|/Script/Engine.CharacterMovementComponent|SetMaxWalkSpeed (Variables|Character|GetCharacterMovement) (Variables|Default|GetOutOfRangeMovementSpeed))))))))

(fn ConstructionScript
  (|CallParentFunction))

(fn LineTracetoTarget
  (bind _capsulecomponent (Variables|Default|GetCapsuleComponent))
  (bind _target (Variables|Default|GetTarget))
  (bind _returnvalue (Transformation|GetWorldLocation _capsulecomponent))
  (bind _rootcomponent (Variables|/Script/Engine.Actor|GetRootComponent _target))
  (bind _returnvalue_2 (Transformation|GetWorldLocation _rootcomponent))
  (Variables|Default|SetDistanceToTarget (Math|Vector|Distance(Vector) _returnvalue _returnvalue_2))
  (bind (_outhit _returnvalue_3) (Collision|LineTraceByChannel _returnvalue _returnvalue_2 "TraceTypeQuery2" false 0 "None"))
  (return _outhit _returnvalue_3))

(fn FireProjectile
  (bind _capsulecomponent (Variables|Default|GetCapsuleComponent))
  (bind _target (Variables|Default|GetTarget))
  (bind _returnvalue (Transformation|GetWorldLocation _capsulecomponent))
  (bind _rootcomponent (Variables|/Script/Engine.Actor|GetRootComponent _target))
  (bind _returnvalue_2 (Transformation|GetWorldLocation _rootcomponent))
  (bind _returnvalue_3 (Game|SpawnActorfromClass "/Game/Blueprints/Enemies/Projectiles/BruteProjectile.BruteProjectile_C" (Math|Transform|MakeTransform _returnvalue (Math|Rotator|FindLookatRotation _returnvalue _returnvalue_2) "1,1,1") "AlwaysSpawn" 0 0))
  (Physics|SetPhysicsLinearVelocity (Variables|/Game/Blueprints/Enemies/Projectiles/BruteProjectile.BruteProjectile_C|GetSphere _returnvalue_3) (* (Math|Vector|GetUnitDirection(Vector) _returnvalue _returnvalue_2) (Variables|Default|GetProjectileSpeed)) false "None")
  (Variables|Default|SetFireProjectileTimer 10))