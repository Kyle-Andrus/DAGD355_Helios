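; Weapon pickup actor, named for the AR, that grants a weapon or ammo to the player character on overlap.
; Collision overlap spawns the collect effect before the player cast, so any overlapping actor triggers it.
; For a player, it searches WeaponsAvailable for its WeaponType, gives ammo on a match or the weapon with ammo otherwise, then destroys itself.
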(event OnComponentBeginOverlap(Collision)
  (params (OverlappedComponent :type Primitive%20Component%20Object%20Reference) (OtherActor :type Actor%20Object%20Reference) (OtherComp :type Primitive%20Component%20Object%20Reference) (OtherBodyIndex :type Integer) (bFromSweep :type Boolean) (SweepResult :type Hit%20Result%20Structure%20%28by%20ref%29))
  (bind _weapontype (Variables|Default|GetweaponType))
  (bind _ammoamount (Variables|Default|GetammoAmount))
  (Niagara|SpawnSystematLocation "/Game/Art/Effect/Collect_Pickup_FX/FX_Collect_Pickup.FX_Collect_Pickup" (Transformation|GetActorLocation))
  (bind _asplayer_character (Utilities|Casting|CastToplayerCharacter OtherActor))
  (bind _index (Utilities|FlowControl|ForLoopwithBreak 0 (- (Utilities|Array|Length (Variables|/Game/Blueprints/Player/playerCharacter.playerCharacter_C|GetweaponsAvailable _asplayer_character)) 1) :!label _label)
    (:LoopBody
      (if (Utilities|Enum|Equal(Enum) (Utilities|Array|Get(acopy) (Variables|/Game/Blueprints/Player/playerCharacter.playerCharacter_C|GetweaponsAvailable _asplayer_character) _index) _weapontype)
        (Default|GiveAmmo _asplayer_character _weapontype _ammoamount)
        (Variables|Default|SetammoApplied true)
        (goto _label Break)))
    (:Completed
      (if (Variables|Default|GetammoApplied)
        _
        (else
          (Default|GiveWeapon _asplayer_character _weapontype _ammoamount)))
      (Actor|DestroyActor))))

(fn ConstructionScript)